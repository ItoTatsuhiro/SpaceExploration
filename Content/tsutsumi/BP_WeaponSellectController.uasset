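; Player controller for a weapon selection screen that shows the mouse cursor and displays the stats of the weapon under it.
; BeginPlay adds the selection and heal widgets to the viewport.
; Each tick, a cursor trace casts the hit actor to WeaponBase and pushes its name, level, HP, speed and attack to the selection widget.
; Defense display is disconnected, and left click only checks weapon validity without acting.
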(event EventBeginPlay
  (Variables|Default|SetbShowMouseCursor true)
  (bind _returnvalue (UserInterface|CreateWidget "/Game/tsutsumi/BP_SelectInterface.BP_SelectInterface_C"))
  (bind _output_get (Variables|Default|SetWidget _returnvalue))
  (UserInterface|Viewport|AddtoViewport _output_get 0)
  (bind _returnvalue_2 (UserInterface|CreateWidget "/Game/tsutsumi/BP_Heal.BP_Heal_C"))
  (UserInterface|Viewport|AddtoViewport _returnvalue_2 0))

(event EventTick
  (params (DeltaSeconds :type Float%20%28single-precision%29))
  (bind _hitresult (Game|Player|GetHitResultUnderCursorbyChannel "TraceTypeQuery1" true))
  (bind _hitactor (Collision|BreakHitResult _hitresult))
  (if (Utilities|IsValid _hitactor)
    (bind _asweapon_base (Utilities|Casting|CastToWeaponBase _hitactor))
    (Default|SetWeaponName (Variables|Default|GetWidget) (.PlayerName (Utilities|Struct|BreakStatus (Variables|/Script/SpaceExploration.WeaponBase|GetWeaponStatus _asweapon_base))))
    (Default|GetWeaponLevelText (Variables|Default|GetWidget) (Utilities|String|ToString(Integer) (.PlayerLevel (Utilities|Struct|BreakStatus (Variables|/Script/SpaceExploration.WeaponBase|GetWeaponStatus _asweapon_base)))))
    (Default|GetWeaponHp (Variables|Default|GetWidget) (Utilities|String|ToString(Float) (.HP (Utilities|Struct|BreakStatus (Variables|/Script/SpaceExploration.WeaponBase|GetWeaponStatus _asweapon_base)))))
    (Default|GetWeaponSpeedText (Variables|Default|GetWidget) (Utilities|String|ToString(Float) (.Speed (Utilities|Struct|BreakStatus (Variables|/Script/SpaceExploration.WeaponBase|GetWeaponStatus _asweapon_base)))))
    (Default|GetWeaponAttackPowerText (Variables|Default|GetWidget) (Utilities|String|ToString(Float) (.AttackPower (Utilities|Struct|BreakStatus (Variables|/Script/SpaceExploration.WeaponBase|GetWeaponStatus _asweapon_base)))))))

(event Input|MouseEvents|LeftMouseButton
  (params (Key :type Key%20Structure :default "None"))
  (:Pressed
    (if (Utilities|IsValid (stale EventTick _asweapon_base))
      _)))

(fn ConstructionScript)

(fn SetParentObject
  (params (NewParam :type Actor%20Object%20Reference))
  (Variables|Default|SetObject NewParam))