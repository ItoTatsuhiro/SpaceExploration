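; Treasure box selection actor that detects when the cursor is over a weapon.
; On BeginPlay it spawns and stores a BP_TestActor offset from itself along Y.
; Each Tick it traces under the cursor and, on a WeaponBase hit, sets IsSelected and registers itself as parent object on BP_WeaponSellectController.
; Hitting another actor clears IsSelected, while hitting nothing leaves it unchanged.
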(event EventBeginPlay
  (bind _returnvalue (Game|SpawnActorfromClass "/Game/tsutsumi/BP_TestActor.BP_TestActor_C" (Math|Conversions|ToTransform(Vector) (+ (Transformation|GetActorLocation) "0.000000,50.000000,0.000000")) "Undefined" "MultiplyWithRoot" 0 0))
  (Variables|Default|SetTestActor _returnvalue))

(event EventTick
  (params (DeltaSeconds :type Float%20%28single-precision%29))
  (bind _returnvalue (Game|GetPlayerController 0))
  (bind _hitresult (Game|Player|GetHitResultUnderCursorbyChannel _returnvalue "TraceTypeQuery1" true))
  (bind _hitactor (Collision|BreakHitResult _hitresult))
  (if (Utilities|IsValid _hitactor)
    (Utilities|Casting|CastToWeaponBase _hitactor
      (:then
        (Variables|Default|SetIsSelected true)
        (bind _asbp_weapon_sellect_controller (Utilities|Casting|CastToBP_WeaponSellectController (Game|GetPlayerController 0)))
        (Default|SetParentObject _asbp_weapon_sellect_controller self))
      (:CastFailed
        (Variables|Default|SetIsSelected false)))))

(fn ConstructionScript)